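; BPC_Quest is a quest component that drives the on-screen quest HUD.
; On BeginPlay it creates a WB_QuestHUD widget, stores it and adds it to the viewport.
; Two custom events push the active quest to that widget: one sets the quest name text and makes the HUD visible, the other fills the objectives list from the quest's objective data.
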(event `self.ReceiveBeginPlay`
  (bind _returnvalue (`|CreateWidget` "/Game/Quest_System/WB_QuestHUD.WB_QuestHUD_C"))
  (bind _output_get (set `self.QuestHUDWidget` _returnvalue))
  (`UserWidget.AddToViewport` _output_get 0))

(event `SetActiveQuestText`
  (`TextBlock.SetText` (`/Game/Quest_System/WB_QuestHUD.ActiveQuestText` (`self.QuestHUDWidget`)) (`KismetTextLibrary.Conv_StringToText` (`.Name_6_42180A2E4BE5311DA86F9189D02C513E` (break `/Game/Quest_System/S_Quest` (`self.ActiveQuest`)))))
  (`Widget.SetVisibility` (`self.QuestHUDWidget`) "Visible"))

(event `SetObjective`
  (bind (_activequest_name _activequest_description _activequest_secunday _activequest_completed _activequest_objective) (break `/Game/Quest_System/S_Quest` (`self.ActiveQuest`)))
  (`/Game/Quest_System/WB_QuestHUD.FillObjectives` (`self.QuestHUDWidget`) _activequest_objective))