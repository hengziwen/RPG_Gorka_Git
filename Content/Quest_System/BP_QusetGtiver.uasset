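; Quest giver NPC that the player talks to for quests and can also damage and kill.
; Interacting steps through Dialogue lines in a widget, then opens a quest widget filled from Quests; interacting again closes it.
; An interact prompt shows inside the trigger radius, and it and the HP bar turn toward the camera every tick.
; Damage updates the bar, plays random hit montages and knockback, and ragdolls at zero HP.
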(event `self.ReceiveTick`
  (params (DeltaSeconds :type "Float (single-precision)"))
  (bind _interactwidget (`self.InteractWidget`))
  ; 使显示的UI始终转向玩家
  (`SceneComponent.K2_SetWorldRotation` _interactwidget (`KismetMathLibrary.FindLookAtRotation` (`SceneComponent.K2_GetComponentLocation` _interactwidget) (`SceneComponent.K2_GetComponentLocation` (`Actor.RootComponent` (`GameplayStatics.GetPlayerCameraManager` 0)))) false false)
  (`SceneComponent.K2_SetWorldRotation` (`self.HPBarWidget`) (`KismetMathLibrary.FindLookAtRotation` (`SceneComponent.K2_GetComponentLocation` _interactwidget) (`SceneComponent.K2_GetComponentLocation` (`Actor.RootComponent` (`GameplayStatics.GetPlayerCameraManager` 0)))) false false))

(event `Ragdoll`
  ; 布娃娃系统
  (`|ExecutionSequence`
    (:`then_0`
      (`KismetSystemLibrary.Delay` 2.5)
      (`PrimitiveComponent.SetSimulatePhysics` (`self.Mesh`) true))
    (:`then_1`
      (`KismetSystemLibrary.Delay` 1.5)
      (`GameplayStatics.PlaySoundAtLocation` "/Game/Auido/GruntsOrHit/SC_Death.SC_Death" (`self.K2_GetActorLocation`) (struct) 1.0 1.0 0.0 null null null null)
      (`Widget.SetVisibility` (`self.HPBarWidgeRef`) "Hidden"))))

(event `self.ReceiveAnyDamage`
  (params (Damage :type "Float (single-precision)") (DamageType :type "DamageType Object Reference") (InstigatedBy :type "Controller Object Reference") (DamageCauser :type "Actor Object Reference"))
  ; 受伤和死亡效果
  (set `self.CurHP` (- (`self.CurHP`) Damage))
  (`/Game/UI/WB_DummHP.UpdateHP` (`self.HPBarWidgeRef`) (`self.CurHP`) (`self.MaxHP`))
  (`self.PlayAnimMontage` (`|GetArrayItem` (`self.HitAnim`) (`KismetMathLibrary.RandomIntegerInRange` 0 (- (`KismetArrayLibrary.Array_Length` (`self.HitAnim`)) 1))))
  (bind _asbp_third_person_character (cast `/Game/ThirdPerson/Blueprints/BP_ThirdPersonCharacter` (`GameplayStatics.GetPlayerCharacter` 0)))
  (`self.LaunchCharacter` (* (`KismetMathLibrary.GetForwardVector` (`self.K2_GetActorRotation` _asbp_third_person_character)) 700.0))
  (`GameplayStatics.PlaySoundAtLocation` "/Game/Auido/GruntsOrHit/416839__tonsil5__grunt1-death-pain.416839__tonsil5__grunt1-death-pain" (`self.K2_GetActorLocation`) (struct) (`KismetMathLibrary.RandomFloatInRange` 1.3 1.5) 1.0 0.0 null null null null)
  (if (<= (`self.CurHP`) 0.0)
    (`PrimitiveComponent.SetSimulatePhysics` (`self.Mesh`) true)
    (`GameplayStatics.PlaySoundAtLocation` "/Game/Auido/GruntsOrHit/SC_Death.SC_Death" (`self.K2_GetActorLocation`) (struct) 1.0 1.0 0.0 null null null null)
    (`Widget.SetVisibility` (`self.HPBarWidgeRef`) "Hidden")))

(event `self.TiggerRadius.OnComponentBeginOverlap`
  (params (OverlappedComponent :type "PrimitiveComponent Object Reference") (OtherActor :type "Actor Object Reference") (OtherComp :type "PrimitiveComponent Object Reference") (OtherBodyIndex :type Integer) (bFromSweep :type Boolean) (SweepResult :type "HitResult Structure (by ref)"))
  ; 显示和关闭处决UI
  (cast `/Game/ThirdPerson/Blueprints/BP_ThirdPersonCharacter` OtherActor)
  (`SceneComponent.SetVisibility` (`self.InteractWidget`) true false))

(event `self.TiggerRadius.OnComponentEndOverlap`
  (params (OverlappedComponent :type "PrimitiveComponent Object Reference") (OtherActor :type "Actor Object Reference") (OtherComp :type "PrimitiveComponent Object Reference") (OtherBodyIndex :type Integer))
  ; 显示和关闭处决UI
  (cast `/Game/ThirdPerson/Blueprints/BP_ThirdPersonCharacter` OtherActor)
  (`SceneComponent.SetVisibility` (`self.InteractWidget`) false false))

(event `/Game/Quest_System/BPI_QuestGriver.INT_Interact`
  (bind _returnvalue (`GameplayStatics.GetPlayerController` 0))
  (if (not (`self.WidgetActive`))
    (if (not (`self.DialogueOpened?`))
      (bind _returnvalue_2 (`|CreateWidget` "/Game/Quest_System/WB_QuestGriverDialogue.WB_QuestGriverDialogue_C"))
      (bind _output_get (set `self.DialogueWidget` _returnvalue_2))
      (`UserWidget.AddToViewport` _output_get 0)
      (set `self.DialogueOpened?` true)
      (set `PlayerController.bShowMouseCursor` true _returnvalue)
      (`WidgetBlueprintLibrary.SetInputMode_GameAndUIEx` _returnvalue null))
    (if (<= (`KismetArrayLibrary.Array_Length` (`self.Dialogue`)) (`self.DialogueIndex`))
      (`Widget.RemoveFromParent` (`self.DialogueWidget`))
      (set `self.DialogueOpened?` false)
      (set `self.DialogueIndex` 0)
      (`self.OpenQuestWidget`)
      (else
        (`TextBlock.SetText` (`/Game/Quest_System/WB_QuestGriverDialogue.DialogueText` (`self.DialogueWidget`)) (`KismetTextLibrary.Conv_StringToText` (`|GetArrayItem` (`self.Dialogue`) (`self.DialogueIndex`))))
        (`/Engine/EditorBlueprintResources/StandardMacros.IncrementInt` (`self.DialogueIndex`))))
    (else
      (`self.CloseWidget`))))

(event `self.ReceiveBeginPlay`
  (bind _maxhp (`self.MaxHP`))
  ; 初始化血条
  (bind _aswb_dumm_hp (cast `/Game/UI/WB_DummHP` (`WidgetComponent.GetWidget` (`self.HPBarWidget`))))
  (bind _output_get (set `self.HPBarWidgeRef` _aswb_dumm_hp))
  (set `self.CurHP` _maxhp)
  (`/Game/UI/WB_DummHP.UpdateHP` _output_get (`self.CurHP`) _maxhp))

(event `OpenQuestWidget`
  (bind _returnvalue (`GameplayStatics.GetPlayerController` 0))
  (bind _returnvalue_2 (`|CreateWidget` "/Game/Quest_System/WB_QuestGriver.WB_QuestGriver_C"))
  (bind _output_get (set `self.QuestWidget` _returnvalue_2))
  (`UserWidget.AddToViewport` _output_get 0)
  (set `self.WidgetActive` true)
  (set `PlayerController.bShowMouseCursor` true _returnvalue)
  (`WidgetBlueprintLibrary.SetInputMode_GameAndUIEx` _returnvalue (`self.QuestWidget`))
  (set `/Game/Quest_System/WB_QuestGriver.QuestGriverBP` self (`self.QuestWidget`))
  (for _array_element (`self.Quests`)
    (`/Game/Quest_System/WB_QuestGriver.AddQuest` (`self.QuestWidget`) _array_element)))

(event `CloseWidget`
  (bind _returnvalue (`GameplayStatics.GetPlayerController` 0))
  (`Widget.RemoveFromParent` (`self.QuestWidget`))
  (set `self.QuestWidget` null)
  (set `self.WidgetActive` false)
  (set `PlayerController.bShowMouseCursor` false _returnvalue)
  (`WidgetBlueprintLibrary.SetInputMode_GameOnly` _returnvalue))

(fn `UserConstructionScript`)