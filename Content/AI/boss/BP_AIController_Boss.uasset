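; BP_AIController_Boss is the AI controller for a boss, running the BT_AI_Boss behavior tree from BeginPlay.
; ActivateBossCombat creates a WB_BossHPBar widget and adds it to the viewport, and DeactivateBossCombat removes it and clears the reference.
; While that widget is valid, Tick pushes the current and max HP into it every frame.
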(event `self.ReceiveBeginPlay`
  (`self.RunBehaviorTree` "/Game/AI/boss/BT_AI_Boss.BT_AI_Boss"))

(event `self.ReceiveTick`
  (params (DeltaSeconds :type "Float (single-precision)"))
  (bind _bosshpbar (`self.BossHPBar`)
    (:`then`
      (`/Game/UI/WB_BossHPBar.UpdateHP` _bosshpbar (`self.Cur HP`) (`self.Max HP`)))
    (:`else`)))

(event `ActivateBossCombat`
  (bind _returnvalue (`|CreateWidget` "/Game/UI/WB_BossHPBar.WB_BossHPBar_C"))
  (bind _output_get (set `self.BossHPBar` _returnvalue))
  (`UserWidget.AddToViewport` _output_get 0))

(event `DeactivateBossCombat`
  (`Widget.RemoveFromParent` (`self.BossHPBar`))
  (set `self.BossHPBar` null))

(fn `UserConstructionScript`
  (`parent.UserConstructionScript`))