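; BP_AI_Boss is the boss AI actor, a thin Blueprint that mirrors its health onto its AI controller.
; Each Tick it casts its controller to BP_AIController_Boss and copies CurHP and MaxHP into it, polling rather than updating on change.
; BeginPlay, Tick and the construction script call their parent versions, and the overlap event is disabled.
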(event `self.ReceiveBeginPlay`
  (`parent.ReceiveBeginPlay`))

(event `self.ReceiveTick`
  (params (DeltaSeconds :type "Float (single-precision)"))
  (`parent.ReceiveTick` DeltaSeconds)
  (bind _asbp_aicontroller_boss (cast `/Game/AI/boss/BP_AIController_Boss` (`AIBlueprintHelperLibrary.GetAIController` self)))
  (set `/Game/AI/boss/BP_AIController_Boss.Cur HP` (`self.CurHP`) _asbp_aicontroller_boss)
  (set `/Game/AI/boss/BP_AIController_Boss.Max HP` (`self.MaxHP`) _asbp_aicontroller_boss))

(fn `UserConstructionScript`
  (`parent.UserConstructionScript`))