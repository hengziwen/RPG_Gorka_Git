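; BP_AI is an enemy character with a health bar that the player can damage or kill with a stealth back assassination.
; Damage updates the HP bar, plays a random hit montage, launches the AI along the player's facing, and ragdolls it at zero HP.
; An overlap shows the assassination prompt, and both widgets face the camera each Tick.
; The stealth interface plays the victim montage, triggers delayed ragdoll, and returns the attacker's alignment location and rotation.
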(event `Ragdoll`
  (`|ExecutionSequence`
    (:`then_0`
      (`KismetSystemLibrary.Delay` 2.5)
      (`PrimitiveComponent.SetSimulatePhysics` (`self.Mesh`) true))
    (:`then_1`
      (`KismetSystemLibrary.Delay` 1.5)
      (`GameplayStatics.PlaySoundAtLocation` "/Game/Auido/GruntsOrHit/SC_Death.SC_Death" (`self.K2_GetActorLocation`) (struct) 1.0 1.0 0.0 null null null null)
      (`Widget.SetVisibility` (`self.HPBarWidgeRef`) "Hidden"))))

(event `self.AssasinaeWidget.OnComponentBeginOverlap`
  (params (OverlappedComponent :type "PrimitiveComponent Object Reference") (OtherActor :type "Actor Object Reference") (OtherComp :type "PrimitiveComponent Object Reference") (OtherBodyIndex :type Integer) (bFromSweep :type Boolean) (SweepResult :type "HitResult Structure (by ref)"))
  (cast `/Game/ThirdPerson/Blueprints/BP_ThirdPersonCharacter` OtherActor)
  (`SceneComponent.SetVisibility` (`self.AssasinaeWidget`) true false))

(event `self.AssasinaeWidget.OnComponentEndOverlap`
  (params (OverlappedComponent :type "PrimitiveComponent Object Reference") (OtherActor :type "Actor Object Reference") (OtherComp :type "PrimitiveComponent Object Reference") (OtherBodyIndex :type Integer))
  (cast `/Game/ThirdPerson/Blueprints/BP_ThirdPersonCharacter` OtherActor)
  (`SceneComponent.SetVisibility` (`self.AssasinaeWidget`) false false))

(event `self.ReceiveTick`
  (params (DeltaSeconds :type "Float (single-precision)"))
  (bind _assasinaewidget (`self.AssasinaeWidget`))
  (`SceneComponent.K2_SetWorldRotation` _assasinaewidget (`KismetMathLibrary.FindLookAtRotation` (`SceneComponent.K2_GetComponentLocation` _assasinaewidget) (`SceneComponent.K2_GetComponentLocation` (`Actor.RootComponent` (`GameplayStatics.GetPlayerCameraManager` 0)))) false false)
  (`SceneComponent.K2_SetWorldRotation` (`self.HPBarWidget`) (`KismetMathLibrary.FindLookAtRotation` (`SceneComponent.K2_GetComponentLocation` _assasinaewidget) (`SceneComponent.K2_GetComponentLocation` (`Actor.RootComponent` (`GameplayStatics.GetPlayerCameraManager` 0)))) false false))

(event `self.ReceiveAnyDamage`
  (params (Damage :type "Float (single-precision)") (DamageType :type "DamageType Object Reference") (InstigatedBy :type "Controller Object Reference") (DamageCauser :type "Actor Object Reference"))
  (set `self.CurHP` (- (`self.CurHP`) Damage))
  (`/Game/UI/WB_DummHP.UpdateHP` (`self.HPBarWidgeRef`) (`self.CurHP`) (`self.MaxHP`))
  (`self.PlayAnimMontage` (`|GetArrayItem` (`self.HitAnim`) (`KismetMathLibrary.RandomIntegerInRange` 0 (- (`KismetArrayLibrary.Array_Length` (`self.HitAnim`)) 1))))
  (bind _asbp_third_person_character (cast `/Game/ThirdPerson/Blueprints/BP_ThirdPersonCharacter` (`GameplayStatics.GetPlayerCharacter` 0)))
  (`self.LaunchCharacter` (* (`KismetMathLibrary.GetForwardVector` (`self.K2_GetActorRotation` _asbp_third_person_character)) 700.0))
  (`GameplayStatics.PlaySoundAtLocation` "/Game/Auido/GruntsOrHit/416839__tonsil5__grunt1-death-pain.416839__tonsil5__grunt1-death-pain" (`self.K2_GetActorLocation`) (struct) (`KismetMathLibrary.RandomFloatInRange` 1.3 1.5) 1.0 0.0 null null null null)
  (if (<= (`self.CurHP`) 0.0)
    (`PrimitiveComponent.SetSimulatePhysics` (`self.Mesh`) true)
    (`GameplayStatics.PlaySoundAtLocation` "/Game/Auido/GruntsOrHit/SC_Death.SC_Death" (`self.K2_GetActorLocation`) (struct) 1.0 1.0 0.0 null null null null)
    (`Widget.SetVisibility` (`self.HPBarWidgeRef`) "Hidden")))

(event `self.ReceiveBeginPlay`
  (bind _maxhp (`self.MaxHP`))
  (bind _aswb_dumm_hp (cast `/Game/UI/WB_DummHP` (`WidgetComponent.GetWidget` (`self.HPBarWidget`))))
  (bind _output_get (set `self.HPBarWidgeRef` _aswb_dumm_hp))
  (set `self.CurHP` _maxhp)
  (`/Game/UI/WB_DummHP.UpdateHP` _output_get (`self.CurHP`) _maxhp))

(fn `INT_StealthBackAssasin`
  (returns (RefLocation :type "Vector Structure") (`Assasin Rotation` :type "Rotator Structure"))
  (`self.PlayAnimMontage` "/Game/Characters/RPG_Characters/Animations/Assasinations/Paired_Knife_Stealth_KidneyAndNeck_Vic_Montage.Paired_Knife_Stealth_KidneyAndNeck_Vic_Montage")
  (`self.Ragdoll`)
  (`SceneComponent.SetVisibility` (`self.AssasinaeWidget`) false false)
  (return (`SceneComponent.K2_GetComponentLocation` (`self.AssasinRef`)) (`self.K2_GetActorRotation`)))

(fn `UserConstructionScript`)