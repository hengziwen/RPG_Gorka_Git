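; BP_AIController_Generic is a generic AI controller that sets the target its AI detects and chases.
; It runs the BT_AI behavior tree on BeginPlay and feeds it through the TargetActor blackboard key from AI Perception updates.
; A successful sight stimulus stores the sensed actor as the target, a non-sight stimulus clears it, and a failed sight stimulus leaves it unchanged.
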(event `self.ReceiveBeginPlay`
  (`self.RunBehaviorTree` "/Game/AI/BT_AI.BT_AI"))

(event `self.AIPerception.OnTargetPerceptionUpdated`
  (params (Actor :type "Actor Object Reference") (Stimulus :type "AIStimulus Structure"))
  ; 检测并追逐目标
  (bind _returnvalue (`AIPerceptionSystem.GetSenseClassForStimulus` Stimulus))
  (if (== _returnvalue "/Script/AIModule.AISense_Sight")
    (if (`.bSuccessfullySensed` (break `AIStimulus` Stimulus))
      (`BlackboardComponent.SetValueAsObject` (`AIBlueprintHelperLibrary.GetBlackboard` null) "TargetActor" Actor))
    (else
      (`BlackboardComponent.SetValueAsObject` (`AIBlueprintHelperLibrary.GetBlackboard` null) "TargetActor" null))))

(fn `UserConstructionScript`)