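; Player status component that tracks current and maximum HP and SP for the owning BP_ThirdPersonCharacter, starting both full on BeginPlay.
; HPChange and SpChange add a signed delta, cap at max, update the character's HUD widget and return true on depletion.
; SpChange updates the HUD before clamping to zero.
; IncreaseLevel refills HP and refreshes its display, but its max HP and SP increments are currently zero.
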(event `self.ReceiveBeginPlay`
  (bind _asbp_third_person_character (cast `/Game/ThirdPerson/Blueprints/BP_ThirdPersonCharacter` (`self.GetOwner`)))
  (set `self.BPCharacterRef` _asbp_third_person_character)
  (set `self.CurHP` (`self.MaxHP`))
  (set `self.CurSP` (`self.MaxSP`)))

(fn `HPChange`
  (params (Demage :type "Float (double-precision)"))
  (returns (isDead :type Boolean))
  (bind _maxhp (`self.MaxHP`))
  (set `self.CurHP` (+ Demage (`self.CurHP`)))
  (`|ExecutionSequence`
    (:`then_0`
      (if (> (`self.CurHP`) _maxhp)
        (set `self.CurHP` _maxhp)))
    (:`then_1`
      (if (<= (`self.CurHP`) 0.0)
        (set `self.CurHP` 0.0)
        (`/Game/UI/WB_HUD.UpdateHP` (`/Game/ThirdPerson/Blueprints/BP_ThirdPersonCharacter.HUDWidget` (`self.BPCharacterRef`)) (`self.CurHP`) (`self.MaxHP`))
        (return true)
        (else
          (`/Game/UI/WB_HUD.UpdateHP` (`/Game/ThirdPerson/Blueprints/BP_ThirdPersonCharacter.HUDWidget` (`self.BPCharacterRef`)) (`self.CurHP`) (`self.MaxHP`))
          (return false))))))

(fn `IncreaseLevel`
  (bind _output_get (set `self.MaxHP` (+ 0.0 (`self.MaxHP`))))
  (set `self.CurHP` _output_get)
  (`/Game/UI/WB_HUD.UpdateHP` (`/Game/ThirdPerson/Blueprints/BP_ThirdPersonCharacter.HUDWidget` (`self.BPCharacterRef`)) (`self.CurHP`) (`self.MaxHP`))
  (set `self.MaxSP` (+ 0.0 (`self.MaxSP`))))

(fn `SpChange`
  (params (CastSP :type "Float (double-precision)"))
  (returns (isExhausted :type Boolean))
  (bind _maxsp (`self.MaxSP`))
  (set `self.CurSP` (+ CastSP (`self.CurSP`)))
  (`|ExecutionSequence`
    (:`then_0`
      (if (> (`self.CurSP`) _maxsp)
        (set `self.CurSP` _maxsp)))
    (:`then_1`
      (`/Game/UI/WB_HUD.UpdateSP` (`/Game/ThirdPerson/Blueprints/BP_ThirdPersonCharacter.HUDWidget` (`self.BPCharacterRef`)) (`self.CurSP`) (`self.MaxSP`))
      (if (<= (`self.CurSP`) 0.0)
        (set `self.CurSP` 0.0)
        (return true)
        (else
          (return false))))))